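; Core game mode that tracks connected player controllers through login, logout and controller swaps during seamless travel.
; Each change prints or triggers a player-list update, which after a short safety delay tells BP_Core_GS to refresh once replication should have finished.
; It also kicks players by list index through BP_Core_PC and runs ServerTravel to a named level via console command.
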(event `self.K2_PostLogin`
  (params (NewPlayer :type "PlayerController Object Reference"))
  ;[1 1 1] Called once player has connected.
  (`KismetArrayLibrary.Array_Add` (`self.ConnectedPlayers`) NewPlayer)
  (`KismetSystemLibrary.PrintText` (`|FormatText` "OnPostLogin: {username}" (`PlayerState.GetPlayerName` (`Controller.PlayerState` NewPlayer))) true true (struct :`G` 0.66 :`B` 1.0 :`A` 1.0) 5.0)
  (`self.Update_PlayerList` :!label _label))

(event `Update_PlayerList`
  ;[1 1 1] Inform clients that the GameState player array should have been replicated. (Delay is for safety)
  (`KismetSystemLibrary.Delay` 0.3)
  (`/Game/_Project/Core/BP_Core_GS.Update_PlayerList` (cast `/Game/_Project/Core/BP_Core_GS` (`GameplayStatics.GetGameState`) :!pure true)))

(event `self.K2_OnLogout`
  (params (ExitingController :type "Controller Object Reference"))
  (bind _asplayer_controller (cast `PlayerController` ExitingController :!pure true))
  ;[1 1 1] Called when player is disconnecting
  (`KismetArrayLibrary.Array_RemoveItem` (`self.ConnectedPlayers`) _asplayer_controller)
  (`KismetSystemLibrary.PrintText` (`|FormatText` "OnLogout: {username}" (`PlayerState.GetPlayerName` (`Controller.PlayerState` _asplayer_controller))) true true (struct :`G` 0.66 :`B` 1.0 :`A` 1.0) 5.0)
  (goto _label))

(event `self.K2_OnSwapPlayerControllers`
  (params (OldPC :type "PlayerController Object Reference") (NewPC :type "PlayerController Object Reference"))
  ;[1 1 1] When PCs are swapped during seamless travel
  (`KismetArrayLibrary.Array_Add` (`self.ConnectedPlayers`) NewPC)
  (goto _label))

(event `ServerTravel`
  (params (LevelName :type Name))
  (`KismetSystemLibrary.ExecuteConsoleCommand` (`KismetTextLibrary.Conv_TextToString` (`|FormatText` "ServerTravel {LevelName}" LevelName)) null))

(fn `KickPlayer`
  (params (`Player Id` :type Integer))
  (`/Game/_Project/Core/BP_Core_PC.OwningClient_KickPlayer` (cast `/Game/_Project/Core/BP_Core_PC` (`|GetArrayItem` (`self.ConnectedPlayers`) `Player Id`) :!pure true)))

(fn `UserConstructionScript`)