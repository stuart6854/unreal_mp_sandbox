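; BP_Core_Hud is the HUD Blueprint that puts the player list and server travel widgets on screen.
; On BeginPlay it creates WBP_PlayerList and WBP_ServerTravel, adds both to the viewport, and keeps a reference to the travel widget.
; Toggle_ServerTravel switches that widget between Collapsed and SelfHitTestInvisible based on its current visibility.
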(event `self.ReceiveBeginPlay`
  (bind _returnvalue (`|CreateWidget` "/Game/_Project/Widgets/WBP_PlayerList.WBP_PlayerList_C"))
  (`UserWidget.AddToViewport` _returnvalue 0)
  (bind _returnvalue_2 (`|CreateWidget` "/Game/_Project/Widgets/WBP_ServerTravel.WBP_ServerTravel_C"))
  (bind _output_get (set `self.ServerTravelWidget` _returnvalue_2))
  (`UserWidget.AddToViewport` _output_get 0))

(event `Toggle_ServerTravel`
  (if (`Widget.IsVisible` (`self.ServerTravelWidget`))
    (`Widget.SetVisibility` (`self.ServerTravelWidget`) "Collapsed")
    (else
      (`Widget.SetVisibility` (`self.ServerTravelWidget`) "SelfHitTestInvisible"))))

(fn `UserConstructionScript`)